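; BP_Statue is a collectible statue that the player picks up by overlap, and it expires after a level-scaled lifetime.
; Overlap with the player notifies BP_ThirdPersonGameMode, while a Tick-driven Delay of default duration minus current level handles expiry.
; Both paths run DestroyStatue, which calls OnPickedUp before destroying the actor, so timeouts fire it too.
; A timeline started on BeginPlay bobs the marker vertically.
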(event OnComponentBeginOverlap(Collider)
  (params (OverlappedComponent :type Primitive%20Component%20Object%20Reference) (OtherActor :type Actor%20Object%20Reference) (OtherComp :type Primitive%20Component%20Object%20Reference) (OtherBodyIndex :type Integer) (bFromSweep :type Boolean) (SweepResult :type Hit%20Result%20Structure%20%28by%20ref%29))
  ;[0.1196 1 0] When Player Picks up Statue
  ;;[1 1 1] Check collision with Player?
  (if (== OtherActor (Game|GetPlayerCharacter 0))
    (bind _asbp_third_person_game_mode (Utilities|Casting|CastToBP_ThirdPersonGameMode (Game|GetGameMode)))
    (Default|OnStatueCollected _asbp_third_person_game_mode)
    (CallFunction|DestroyStatue)))

(event Custom|Destroy%20Statue
  ;[0.08501 1 0] Custom event to Destroy statue
  (Default|CallONPickedUp)
  (Actor|DestroyActor))

(event EventBeginPlay
  ;[0.1154 1 0] Statue Pointer Bouncing
  (bind _bounce (Timeline|PointerBounce PlayFromStart)
    (:Update
      (Transformation|SetRelativeLocation (Variables|Default|GetStatueMarker) (Math|Vector|MakeVector 0.0 0.0 _bounce) false false))))

(event EventTick
  (params (DeltaSeconds :type Float%20%28single-precision%29))
  ;[0.05829 1 0] Statue Active Duration
  (bind _asbp_third_person_game_mode (Utilities|Casting|CastToBP_ThirdPersonGameMode (Game|GetGameMode)))
  (bind _output_get (Variables|Default|SetStatueActiveDuration (- (Variables|Default|GetDefaultDuration) (Variables|/Game/ThirdPerson/Blueprints/BP_ThirdPersonGameMode.BP_ThirdPersonGameMode_C|GetCurrentLevel _asbp_third_person_game_mode))))
  (Utilities|FlowControl|Delay (Math|Conversions|ToFloat(Integer) _output_get))
  (CallFunction|DestroyStatue))

(fn ConstructionScript)