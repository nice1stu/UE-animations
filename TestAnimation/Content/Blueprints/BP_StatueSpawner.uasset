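; BP_StatueSpawner keeps a population of BP_Statue pickups scattered around itself, starting with MaxStatues at BeginPlay.
; Each statue spawns at a random X/Y offset within a square around the spawner at its height, adjusting for collisions.
; It binds to each statue's picked-up event to spawn a replacement, and retries after a short delay if spawning fails.
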(event Custom|Spawn%20Statue
  (bind _returnvalue (Transformation|GetActorLocation))
  ;[0.1692 1 0] Spawn Statue at Random Location
  (Development|PrintString "Spawn Statue +1")
  (bind _output_get (Variables|Default|SetStatueSpawnLocation (Math|Vector|MakeVector (+ (.x _returnvalue) (Math|Random|RandomFloatinRange -1.5e+03 1.5e+03)) (+ (.y _returnvalue) (Math|Random|RandomFloatinRange -1.5e+03 1.5e+03)) (.z _returnvalue))))
  (bind _returnvalue_2 (Game|SpawnActorfromClass "/Game/Blueprints/BP_Statue.BP_Statue_C" (Math|Conversions|ToTransform(Vector) _output_get) "AdjustIfPossibleButAlwaysSpawn" "MultiplyWithRoot" 0 0)) ; Adjusting location but always spawn does not work
  (if (Utilities|IsValid _returnvalue_2)
    (EventDispatchers|BindEventtoONPickedUp _returnvalue_2 (delegate Custom|OnStatuePickedUp))
    (else
      (Utilities|FlowControl|Delay 0.1)
      (Development|PrintString "Fail to spawn" true true "(R=1.000000,G=0.003003,B=0.000000,A=1.000000)")
      (CallFunction|SpawnStatue))))

(event Custom|OnStatuePickedUp
  ;[0.1692 1 0] Spawn Statue at Random Location
  (CallFunction|SpawnStatue))

(event EventBeginPlay
  ;[0.1166 1 0] Start game with Max # Statues in game
  (for _index (range 1 (Variables|Default|GetMax#Statues))
    (CallFunction|SpawnStatue)))

(fn ConstructionScript)